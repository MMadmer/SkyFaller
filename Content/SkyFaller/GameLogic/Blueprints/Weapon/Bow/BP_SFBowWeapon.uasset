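; Bow weapon Blueprint for SkyFaller that adds charge haptics, shot audio and shadow toggling on top of its parent weapon logic.
; Starting fire plays charging feedback only when the owner is not falling, with intensity driven by a haptic strength curve as charge changes, and stopping fire ends it.
; A successful shot plays audio, and the mesh casts shadows only after being dropped, not while set as the weapon.
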(event `self.ReceiveBeginPlay`
  (add `self.OnChargeChanged` (delegate `ChargeChanged`)))

(event `ChargeChanged` :!signature `self.OnChargeChanged`
  (params (ChargeNorm :type "Float (double-precision)"))
  (bind _hapticstrenght (`self.HapticStrenght`)
    (:`then`
      (`ForceFeedbackComponent.SetIntensityMultiplier` (`self.ChargingFeedback`) (`CurveFloat.GetFloatValue` _hapticstrenght ChargeNorm)))
    (:`else`)))

(event `self.StartFire`
  (bind _chargingfeedback (`self.ChargingFeedback`))
  (bind _returnvalue (`self.GetComponentByClass` (`self.GetOwner`) "/Script/Engine.PawnMovementComponent"))
  (`parent.StartFire`)
  (`/Engine/EditorBlueprintResources/StandardMacros.IsValid` _returnvalue
    (:`Is Valid`
      (if (not (`NavMovementComponent.IsFalling` _returnvalue))
        (bind _hapticstrenght (`self.HapticStrenght`)
          (:`then`
            (`ForceFeedbackComponent.SetIntensityMultiplier` _chargingfeedback (`CurveFloat.GetFloatValue` _hapticstrenght 0.0))
            (`ForceFeedbackComponent.Play` _chargingfeedback 0.0))
          (:`else`))))))

(event `self.StopFire`
  (`parent.StopFire`)
  (`ForceFeedbackComponent.Stop` (`self.ChargingFeedback`)))

(event `self.OnWeaponSet`
  (`parent.OnWeaponSet`)
  (`PrimitiveComponent.SetCastShadow` (`self.WeaponMesh`) false))

(event `self.OnWeaponDrop`
  (`parent.OnWeaponDrop`)
  (`PrimitiveComponent.SetCastShadow` (`self.WeaponMesh`) true))

(fn `MakeShot`
  (returns (ReturnValue :type Boolean))
  (locals (EndLoc :type "Vector Structure") (Direction :type "Vector Structure"))
  (bind _returnvalue (`parent.MakeShot`))
  (if _returnvalue
    (`AudioComponent.Play` (`self.ShotAudio`) 0.0)
    (return true)
    (else
      (return false))))

(fn `UserConstructionScript`)