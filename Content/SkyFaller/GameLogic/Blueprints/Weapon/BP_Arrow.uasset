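; BP_Arrow is an arrow projectile that sticks into the first actor it overlaps, ignoring its owner and instigator.
; The construction script sizes its collision box from the mesh bounds, with adjustable cross-section scale.
; On hit it attaches, stops trail and movement, and plays a sound except on SFTrap actors.
; It then teleports forward to fake penetration and, after a short delay, applies mass-scaled velocity impulse to physics-simulating components.
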(event `self.ReceiveBeginPlay`
  (bind _collisionbox (`self.CollisionBox`))
  (`self.SetLifeSpan` (`self.Lifetime`))
  (`PrimitiveComponent.IgnoreActorWhenMoving` _collisionbox (`self.GetOwner`) true)
  (`PrimitiveComponent.IgnoreActorWhenMoving` _collisionbox (`self.GetInstigator`) true))

(event `self.CollisionBox.OnComponentBeginOverlap`
  (params (OverlappedComponent :type "PrimitiveComponent Object Reference") (OtherActor :type "Actor Object Reference") (OtherComp :type "PrimitiveComponent Object Reference") (OtherBodyIndex :type Integer) (bFromSweep :type Boolean) (SweepResult :type "HitResult Structure (by ref)"))
  (bind (_bblockinghit _binitialoverlap _time _distance _location _impactpoint) (`GameplayStatics.BreakHitResult` SweepResult))
  (if (and (!= OtherActor (`self.GetOwner`)) (!= OtherActor (`self.GetInstigator`)))
    (`/Engine/EditorBlueprintResources/StandardMacros.DoOnce` false
      (:`Completed`
        (`PrimitiveComponent.SetCollisionEnabled` (`self.CollisionBox`) "NoCollision")
        (`self.K2_AttachToActor` OtherActor "None" "KeepWorld" "KeepWorld" "KeepWorld")
        (`ActorComponent.Deactivate` (`self.TraceFX`))
        (`|ExecutionSequence`
          (:`then_0`
            (cast `SFTrap` OtherActor
              (:`CastFailed`
                (`GameplayStatics.PlaySoundAtLocation` (`self.HitSound`) _impactpoint (struct) 1.0 1.0 0.0 "/Game/SkyFaller/GameLogic/Audio/SA_far.SA_Far" null null))))
          (:`then_1`
            (set `self.CachedVelocity` (`MovementComponent.Velocity` (`self.ProjectileMovement`)))
            (`ActorComponent.Deactivate` (`self.ProjectileMovement`))
            (`self.Penetrate`)
            (`KismetSystemLibrary.Delay` 0.016667)
            (`/Engine/EditorBlueprintResources/StandardMacros.IsValid` OtherComp
              (:`Is Valid`
                (if (`SceneComponent.IsSimulatingPhysics` OtherComp "None")
                  (`PrimitiveComponent.AddImpulseAtLocation` OtherComp (* (`self.CachedVelocity`) (`self.Mass`)) _impactpoint "None"))))))))))

(fn `Penetrate`
  (bind _boxextent_x (`KismetMathLibrary.BreakVector` (`BoxComponent.BoxExtent` (`self.CollisionBox`))))
  (`self.K2_SetActorLocation` (+ (`self.K2_GetActorLocation`) (* (`self.GetActorForwardVector`) (* _boxextent_x 2.0 (`self.MaxPenetrationNorm`)))) false true))

(fn `UserConstructionScript`
  (bind (_origin _boxextent) (`KismetSystemLibrary.GetComponentBounds` (`self.ArrowMesh`)))
  (`BoxComponent.SetBoxExtent` (`self.CollisionBox`) (`KismetMathLibrary.MakeVector` (.x _boxextent) (* (.y _boxextent) (`self.CollisionScale`)) (* (.z _boxextent) (`self.CollisionScale`))) false))