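; Base random prop for SkyFaller that varies placed scenery at runtime through spawn chance, mesh, yaw and scale.
; On BeginPlay it destroys itself by DestroyChance percentage, otherwise async-loads a random entry from Meshes while applying random yaw and uniform scale from MinScale to 1.
; An empty list or failed mesh cast also destroys the actor.
; The construction script blocking-loads the first mesh as a preview, which BeginPlay clears.
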(event `self.ReceiveBeginPlay`
  (bind (_returnvalue_roll _returnvalue_pitch) (`KismetMathLibrary.BreakRotator` (`self.K2_GetActorRotation`)))
  (if (> (`KismetMathLibrary.RandomFloatInRange` 0.0 100.0) (`self.DestroyChance`))
    (`StaticMeshComponent.SetStaticMesh` (`self.StaticMesh`) null)
    (bind _result (`BlueprintSetLibrary.Set_ToArray` (`self.Meshes`)))
    (if (`KismetArrayLibrary.Array_IsValidIndex` _result)
      (bind _object (`|LoadAsset` (`KismetArrayLibrary.Array_Random` _result))
        (:`then`
          (`self.K2_SetActorTransform` (`KismetMathLibrary.MakeTransform` (`self.K2_GetActorLocation`) (`KismetMathLibrary.MakeRotator` _returnvalue_roll _returnvalue_pitch (`KismetMathLibrary.RandomFloatInRange` 0.0 360.0)) (`KismetMathLibrary.Conv_DoubleToVector` (`KismetMathLibrary.RandomFloatInRange` (`self.MinScale`) 1.0))) false true))
        (:`Completed`
          (bind _asstatic_mesh (cast `StaticMesh` _object)
            (:`then`
              (`StaticMeshComponent.SetStaticMesh` (`self.StaticMesh`) _asstatic_mesh))
            (:`CastFailed`
              (`self.K2_DestroyActor`)))))
      (else
        (`self.K2_DestroyActor`)))
    (else
      (`self.K2_DestroyActor`))))

(fn `UserConstructionScript`
  (`StaticMeshComponent.SetStaticMesh` (`self.StaticMesh`) null)
  (bind _result (`BlueprintSetLibrary.Set_ToArray` (`self.Meshes`)))
  (if (`KismetArrayLibrary.Array_IsValidIndex` _result)
    (bind _returnvalue (`KismetSystemLibrary.LoadAsset_Blocking` (`|GetArrayItem` _result)))
    (bind _asstatic_mesh (cast `StaticMesh` _returnvalue))
    (`StaticMeshComponent.SetStaticMesh` (`self.StaticMesh`) _asstatic_mesh)))