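; Base player character for SkyFaller, handling first-level controls for movement, looking, jumping and firing.
; Enhanced Input actions drive movement along the actor's forward and right vectors, controller yaw and pitch, and the jump.
; Fire input starts the WeaponComponent on press and stops it on release or cancel, leaving firing logic to that component.
; Landing, reported by the movement component, plays LandFeedback.
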(event `self.ReceiveBeginPlay`)

(event `self.CharacterMovement.OnLanded`
  (`ForceFeedbackComponent.Play` (`self.LandFeedback`) 0.0))

(event `EnhancedInput|/Game/SkyFaller/GameLogic/Input/Actions/IA_Look`
  (params (ActionValue :type "Vector2D Structure") (ElapsedSeconds :type "Float (single-precision)") (TriggeredSeconds :type "Float (single-precision)"))
  (:`Triggered`
    (`self.AddControllerPitchInput` ActionValue_Y)
    (`self.AddControllerYawInput` ActionValue_X)))

(event `EnhancedInput|/Game/SkyFaller/GameLogic/Input/Actions/IA_Fire`
  (params (ActionValue :type Boolean) (ElapsedSeconds :type "Float (single-precision)") (TriggeredSeconds :type "Float (single-precision)"))
  (bind _weaponcomponent (`self.WeaponComponent`))
  (:`Started`
    (`SFWeaponComponent.StartFire` _weaponcomponent))
  (:`Canceled`
    (`SFWeaponComponent.StopFire` _weaponcomponent :!label _label))
  (:`Completed`
    (goto _label)))

(event `EnhancedInput|/Game/SkyFaller/GameLogic/Input/Actions/IA_Move`
  (params (ActionValue :type "Vector2D Structure") (ElapsedSeconds :type "Float (single-precision)") (TriggeredSeconds :type "Float (single-precision)"))
  (:`Triggered`
    (`self.AddMovementInput` (`self.GetActorForwardVector`) ActionValue_Y)
    (`self.AddMovementInput` (`self.GetActorRightVector`) ActionValue_X)))

(event `EnhancedInput|/Game/SkyFaller/GameLogic/Input/Actions/IA_Jump`
  (params (ActionValue :type Boolean) (ElapsedSeconds :type "Float (single-precision)") (TriggeredSeconds :type "Float (single-precision)"))
  (:`Started`
    (`self.Jump`)))

(fn `UserConstructionScript`)